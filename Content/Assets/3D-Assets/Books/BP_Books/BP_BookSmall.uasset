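; BP_BookSmall is a small book prop with a configurable cover color.
; The construction script creates a dynamic material instance on the BookSmall component if none is valid, then writes the HasColor and Color parameters from the actor's variables.
; A helper function converts the HasColor boolean to a scalar for the material.
; The event graph has no runtime logic.
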(event EventBeginPlay)

(event Collision|EventActorBeginOverlap
  (params (OtherActor :type Actor%20Object%20Reference)))

(event EventTick
  (params (DeltaSeconds :type Float%20%28single-precision%29)))

(fn ConstructionScript
  (Utilities|IsValid (Variables|Default|GetMID)
    (:Is%20Valid
      _)
    (:Is%20Not%20Valid
      (bind _returnvalue (Rendering|Material|CreateDynamicMaterialInstance (Variables|Default|GetBook_small) 0 0 "None" :!class /Script/Engine.PrimitiveComponent))
      (Variables|Default|SetMID _returnvalue)))
  (Rendering|Material|SetScalarParameterValue (Variables|Default|GetMID) "HasColor" (CallFunction|Scalarvalueset (Variables|Default|GethasColor)) :!class /Script/Engine.MaterialInstanceDynamic)
  (Rendering|Material|SetVectorParameterValue (Variables|Default|GetMID) "Color" (Variables|Default|GetColor) :!class /Script/Engine.MaterialInstanceDynamic))

(fn Scalarvalueset
  (params (Condition :type Boolean))
  (if Condition
    (Variables|Default|SetScalarValue 1.0)
    (else
      (Variables|Default|SetScalarValue 0.0)))
  (return (Variables|Default|GetScalarValue)))