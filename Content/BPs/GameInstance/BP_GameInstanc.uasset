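; Game instance that owns the player's settings save and applies saved audio volumes at startup.
; On Init it loads or creates the Settings save, then retries each tick until a game mode is valid.
; It then overrides master, music and SFX sound class volumes and pushes the sound mix.
; It writes the save to disk on Shutdown and exposes it through ReturnSettingsSave.
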(event EventInit
  (bind _returnvalue (SaveGame|DoesSaveGameExist "Settings"))
  (if _returnvalue
    (bind _returnvalue_2 (SaveGame|LoadGamefromSlot "Settings"))
    (bind _asbp_settings_save (Utilities|Casting|CastToBP_SettingsSave _returnvalue_2))
    (Variables|Default|SetSettingsSave _asbp_settings_save)
    (else
      (bind _returnvalue_3 (SaveGame|CreateSaveGameObject "/Game/BPs/Settings/BP_SettingsSave.BP_SettingsSave_C"))
      (Variables|Default|SetSettingsSave _returnvalue_3)))
  (Utilities|IsValid (Game|GetGameMode) :!label _label
    (:Is%20Valid
      (Audio|SetSoundMixClassOverride "/Game/Sound/SoundMixer/HTKSoundMix.HTKSoundMix" "/Game/Sound/SoundMixer/HTKMaster.HTKMaster" (Variables|/Game/BPs/Settings/BP_SettingsSave.BP_SettingsSave_C|GetMasterVolume (Variables|Default|GetSettingsSave)) 1.0 0.0 true)
      (Audio|SetSoundMixClassOverride "/Game/Sound/SoundMixer/HTKSoundMix.HTKSoundMix" "/Game/Sound/SoundMixer/HTKMusic.HTKMusic" (Variables|/Game/BPs/Settings/BP_SettingsSave.BP_SettingsSave_C|GetMusicVolume (Variables|Default|GetSettingsSave)) 1.0 0.0 true)
      (Audio|SetSoundMixClassOverride "/Game/Sound/SoundMixer/HTKSoundMix.HTKSoundMix" "/Game/Sound/SoundMixer/HTKSFX.HTKSFX" (Variables|/Game/BPs/Settings/BP_SettingsSave.BP_SettingsSave_C|GetSFXVolume (Variables|Default|GetSettingsSave)) 1.0 0.0 true)
      (Audio|PushSoundMixModifier "/Game/Sound/SoundMixer/HTKSoundMix.HTKSoundMix"))
    (:Is%20Not%20Valid
      (Utilities|FlowControl|DelayUntilNextTick)
      (goto _label))))

(event EventShutdown
  (SaveGame|SaveGametoSlot (Variables|Default|GetSettingsSave) "Settings"))

(fn ReturnSettingsSave
  (return (Variables|Default|GetSettingsSave)))