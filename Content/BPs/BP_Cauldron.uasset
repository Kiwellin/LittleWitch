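; Interactable cauldron where the player delivers collected ingredients.
; On BeginPlay it builds the list of five ingredient types and passes it to the collectible info widgets.
; Interact calls Delivered on the player character's current ingredient, then SequenceOnceDelivered with the cauldron as argument.
; ActivateSequence plays CurrentSequence with player input disabled, then clears it and restores input after a delay matching the sequence's end time.
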(event Custom|ActivateSequence
  (bind _returnvalue (Game|GetPlayerController 0))
  (bind _returnvalue_2 (Game|GetPlayerController 0))
  (Utilities|IsValid (Variables|Default|GetCurrentSequence)
    (:Is%20Valid
      (Input|DisableInput _returnvalue_2 _returnvalue_2)
      (Sequencer|Player|Play (Variables|/Script/LevelSequence.LevelSequenceActor|GetSequencePlayer (Variables|Default|GetCurrentSequence)) :!class /Script/MovieScene.MovieSceneSequencePlayer)
      (bind _returnvalue_3 (Class|MovieSceneSequenceExtensions|GetPlaybackEndSeconds (Class|MovieSceneSequencePlayer|GetSequence (Variables|/Script/LevelSequence.LevelSequenceActor|GetSequencePlayer (Variables|Default|GetCurrentSequence)))))
      (Utilities|FlowControl|Delay _returnvalue_3)
      (Variables|Default|SetCurrentSequence 0)
      (Input|EnableInput _returnvalue _returnvalue))))

(event EventBeginPlay
  (Variables|Default|SetIngredients (Utilities|Array|MakeArray "/Game/BPs/BP_IngredientJar.BP_IngredientJar_C" "/Game/BPs/BP_IngredientMushroom.BP_IngredientMushroom_C" "/Game/BPs/BP_IngredientLiquid.BP_IngredientLiquid_C" "/Game/BPs/BP_IngredientHerbs.BP_IngredientHerbs_C" "/Game/BPs/BP_IngredientRoots.BP_IngredientRoots_C"))
  (bind _asbp_third_person_character (Utilities|Casting|CastToBP_ThirdPersonCharacter (Game|Player|GetPlayerPawn 0)))
  (bind _foundwidgets (Widget|GetAllWidgetsOfClass "/Game/UI/BPW_CollectibleInfo.BPW_CollectibleInfo_C" true))
  (for _array_element _foundwidgets
    (bind _output_get (Variables|Default|SetArray%20Element _array_element))
    (Variables|/Game/UI/BPW_CollectibleInfo.BPW_CollectibleInfo_C|SetIngredientList _output_get (Variables|Default|GetIngredients))))

(event Collision|EventActorBeginOverlap
  (params (OtherActor :type Actor%20Object%20Reference)))

(event EventTick
  (params (DeltaSeconds :type Float%20%28single-precision%29)))

(event EventInteract
  (bind _asbp_third_person_character (Utilities|Casting|CastToBP_ThirdPersonCharacter (Game|Player|GetPlayerPawn 0)))
  (Utilities|IsValid (Variables|/Game/BPs/BP_ThirdPersonCharacter.BP_ThirdPersonCharacter_C|GetIngredient _asbp_third_person_character)
    (:Is%20Valid
      (Default|Delivered (Variables|/Game/BPs/BP_ThirdPersonCharacter.BP_ThirdPersonCharacter_C|GetIngredient _asbp_third_person_character) _asbp_third_person_character)
      (Default|SequenceOnceDelivered (Variables|/Game/BPs/BP_ThirdPersonCharacter.BP_ThirdPersonCharacter_C|GetIngredient _asbp_third_person_character) self))))

(fn ConstructionScript
  (|CallParentFunction))