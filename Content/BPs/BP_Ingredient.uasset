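; BP_Ingredient is a collectible ingredient actor that the player picks up through interaction.
; Interact fires Collected, which plays a 2D sound cue, then stores the ingredient on the third-person character.
; After a short delay it hides the actor and disables mesh collision rather than destroying it.
; Delivered and SequenceOnceDelivered, which receives a cauldron, are empty events here.
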(event Custom|Collected
  (params (ThirdPersonCharacter :type BP%20Third%20Person%20Character%20Object%20Reference))
  (CallFunction|PlaySound))

(event Custom|Delivered
  (params (chara :type BP%20Third%20Person%20Character%20Object%20Reference)))

(event Custom|SequenceOnceDelivered
  (params (Cauldron :type BP%20Cauldron%20Object%20Reference)))

(event Custom|PlaySound
  (Audio|PlaySound2D "/Game/Sound/SFX/pickups/ingredients/IngredientCue.IngredientCue" 1.0 1.0 0.0 0 0))

(event EventBeginPlay)

(event Collision|EventActorBeginOverlap
  (params (OtherActor :type Actor%20Object%20Reference)))

(event EventTick
  (params (DeltaSeconds :type Float%20%28single-precision%29)))

(event EventInteract
  (bind _asbp_third_person_character (Utilities|Casting|CastToBP_ThirdPersonCharacter (Game|Player|GetPlayerPawn 0)))
  (CallFunction|Collected _asbp_third_person_character)
  (Variables|/Game/BPs/BP_ThirdPersonCharacter.BP_ThirdPersonCharacter_C|SetIngredient _asbp_third_person_character self)
  (Utilities|FlowControl|Delay 0.2)
  (Rendering|SetActorHiddenInGame true)
  (Collision|SetCollisionEnabled (Variables|Default|Getmesh) "NoCollision"))

(fn ConstructionScript
  (|CallParentFunction))