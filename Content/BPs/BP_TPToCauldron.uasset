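; BP_TPToCauldron is a labeled trigger actor that changes the player character's respawn point to CauldronRespawn; no teleport happens in this Blueprint.
; On BeginPlay it writes its Text to the TextRender and offsets that label's relative location by AddedHeight.
; Any actor overlap casts player pawn 0 to BP_ThirdPersonCharacter and sets MyRespawnPoint, without checking which actor overlapped.
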(event Collision|EventActorBeginOverlap
  (params (OtherActor :type Actor%20Object%20Reference))
  (bind _asbp_third_person_character (Utilities|Casting|CastToBP_ThirdPersonCharacter (Game|Player|GetPlayerPawn 0)))
  (Variables|/Game/BPs/BP_ThirdPersonCharacter.BP_ThirdPersonCharacter_C|SetMyRespawnPoint _asbp_third_person_character (Variables|Default|GetCauldronRespawn)))

(event EventBeginPlay
  (bind _textrender (Variables|Default|GetTextRender))
  (bind _returnvalue (Transformation|GetRelativeTransform _textrender))
  (Rendering|Components|TextRender|SetText _textrender (Variables|Default|GetText))
  (Transformation|SetRelativeTransform _textrender (Math|Transform|MakeTransform (+ (.location _returnvalue) (Variables|Default|GetAdded%20Height)) (.rotation _returnvalue) (.scale _returnvalue)) false false))

(fn ConstructionScript)