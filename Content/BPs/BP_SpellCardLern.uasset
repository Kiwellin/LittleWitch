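; BP_SpellCardLern is an interactable spell card that teaches the player a Fire or Plant spell, chosen by WhatSpell.
; Interact fires LookAtCard on alternate calls, setting the matching learned flag on the character, zeroing its velocity and switching input to UI only.
; It creates or reuses BP_SpellWidget to animate in the card's sketch.
; StopLooking restores game input and reverses the animation, but nothing in this Blueprint runs it.
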(event Custom|StopLooking
  (Input|SetInputModeGameOnly (Game|GetPlayerController 0) true)
  (Class|UserWidget|PlayAnimationReverse (stale Custom|LookAtCard _output_get) (Variables|/Game/UI/BP_SpellWidget.BP_SpellWidget_C|GetMoveCardUpDown (stale Custom|LookAtCard _output_get)) 1.0 false))

(event Custom|LookAtCard
  (bind _returnvalue (Game|GetPlayerController 0))
  (CallFunction|LearnPlants)
  (CallFunction|LearnFire)
  (Variables|/Script/Engine.MovementComponent|SetVelocity (Variables|/Script/Engine.Character|GetCharacterMovement (Variables|Default|GetTPCharacter)) "0, 0, 0")
  (Input|SetInputModeUIOnly _returnvalue 0 "DoNotLock" true)
  (bind _spellwidget (Variables|Default|GetSpellWidget)
    (:then
      (Appearance|SetBrushfromTexture (Variables|/Game/UI/BP_SpellWidget.BP_SpellWidget_C|GetSpellcardImage _spellwidget) (Utilities|Select :Index (Variables|Default|GetWhatSpell) :NewEnumerator0 "/Game/UI/MaterialsAndTextures/FireCardSketch.FireCardSketch" :NewEnumerator1 "/Game/UI/MaterialsAndTextures/PlantCardSketch.PlantCardSketch") false))
    (:else
      (bind _returnvalue_2 (UserInterface|CreateWidget "/Game/UI/BP_SpellWidget.BP_SpellWidget_C" _returnvalue))
      (bind _output_get (Variables|Default|SetSpellWidget _returnvalue_2))
      (Appearance|SetBrushfromTexture (Variables|/Game/UI/BP_SpellWidget.BP_SpellWidget_C|GetSpellcardImage _output_get) (Utilities|Select :Index (Variables|Default|GetWhatSpell) :NewEnumerator0 "/Game/UI/MaterialsAndTextures/FireCardSketch.FireCardSketch" :NewEnumerator1 "/Game/UI/MaterialsAndTextures/PlantCardSketch.PlantCardSketch") false)
      (UserInterface|Viewport|AddtoPlayerScreen _output_get)))
  (Class|UserWidget|PlayAnimationForward _output_get (Variables|/Game/UI/BP_SpellWidget.BP_SpellWidget_C|GetMoveCardUpDown _output_get) 1.0 false)
  (Utilities|FlowControl|Delay 0.2))

(event EventBeginPlay
  (|CallParentFunction)
  (bind _asbp_third_person_character (Utilities|Casting|CastToBP_ThirdPersonCharacter (Game|Player|GetPlayerPawn 0)))
  (Variables|Default|SetTPCharacter _asbp_third_person_character))

(event Collision|EventActorBeginOverlap
  (params (OtherActor :type Actor%20Object%20Reference))
  (|CallParentFunction OtherActor) ; This node is disabled and will not be called.\nDrag off pins to build functionality.
)

(event EventTick
  (params (DeltaSeconds :type Float%20%28single-precision%29))
  (|CallParentFunction DeltaSeconds) ; This node is disabled and will not be called.\nDrag off pins to build functionality.
)

(event EventInteract
  (Utilities|FlowControl|FlipFlop
    (:A
      (CallFunction|LookatCard))))

(fn ConstructionScript
  (|CallParentFunction))

(fn LearnPlants
  (if (Variables|/Game/BPs/BP_ThirdPersonCharacter.BP_ThirdPersonCharacter_C|GetLearnedPlantSpell (Variables|Default|GetTPCharacter))
    _
    (else
      (Utilities|FlowControl|DoOnce false
        (:Completed
          (Variables|/Game/BPs/BP_ThirdPersonCharacter.BP_ThirdPersonCharacter_C|SetLearnedPlantSpell (Variables|Default|GetTPCharacter) (Utilities|Enum|Equal(Enum) (Variables|Default|GetWhatSpell) "NewEnumerator1"))))))
  (return))

(fn LearnFire
  (bind _tpcharacter (Variables|Default|GetTPCharacter))
  (if (Variables|/Game/BPs/BP_ThirdPersonCharacter.BP_ThirdPersonCharacter_C|GetLearnedFireSpell _tpcharacter)
    _
    (else
      (Utilities|FlowControl|DoOnce false
        (:Completed
          (Variables|/Game/BPs/BP_ThirdPersonCharacter.BP_ThirdPersonCharacter_C|SetLearnedFireSpell _tpcharacter (Utilities|Enum|Equal(Enum) (Variables|Default|GetWhatSpell) "NewEnumerator0"))))))
  (return))