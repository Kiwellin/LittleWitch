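; Book-to-cauldron actor that travels along the spline of an assigned SplineActor, matching its location and rotation.
; BeginPlay sets the starting distance from a normalised offset, or prints a warning if no spline is assigned.
; Each Interact call advances one frame-time step at TravelSpeed, wrapping at either end to loop.
; A separate MoveAlongSpline event instead drives the transform by Timeline alpha over the spline length.
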(event Custom|MoveAlongSpline
  (bind _spline_ (Timeline|Timeline Play)
    (:Update
      (Transformation|SetActorLocation (.Location (CallFunction|GetLocationandRotationfromSpline _spline_)) false false)
      (Transformation|SetActorRotation (.Rotation (CallFunction|GetLocationandRotationfromSpline _spline_))))))

(event EventBeginPlay
  (Utilities|IsValid (Variables|Default|GetSplineActor)
    (:Is%20Valid
      (CallFunction|ApplyStartOffset))
    (:Is%20Not%20Valid
      (Development|PrintString "Spline not assigned"))))

(event Collision|EventActorBeginOverlap
  (params (OtherActor :type Actor%20Object%20Reference)))

(event EventTick
  (params (DeltaSeconds :type Float%20%28single-precision%29)))

(event EventInteract
  (CallFunction|UpdateDistanceAlongSpline)
  (CallFunction|UpdateLocation)
  (CallFunction|UpdateRotation))

(fn ConstructionScript
  (|CallParentFunction))

(fn GetLocationandRotationfromSpline
  (params (A :type Float%20%28double-precision%29))
  (bind _splineactor (Variables|Default|GetSplineActor))
  (bind _spline (Variables|/Game/BPs/BP_SplineActor.BP_SplineActor_C|GetSpline _splineactor))
  (bind _returnvalue (Spline|GetSplineLength _spline))
  (bind _returnvalue_2 (* A _returnvalue))
  (return (Spline|GetLocationatDistanceAlongSpline _spline _returnvalue_2 "World") (Spline|GetRotationatDistanceAlongSpline _spline _returnvalue_2 "World")))

(fn ApplyStartOffset
  (Variables|Default|SetDistanceAlongSpline (* (Variables|Default|GetSpline%20Offset) (Spline|GetSplineLength (Variables|/Game/BPs/BP_SplineActor.BP_SplineActor_C|GetSpline (Variables|Default|GetSplineActor))))))

(fn ClampDistanceAlongSplne
  (params (SplineLength :type Float%20%28double-precision%29))
  (Utilities|FlowControl|Sequence
    (:then_0
      (if (>= (Variables|Default|GetDistanceAlongSpline) SplineLength)
        (Variables|Default|SetDistanceAlongSpline (- (Variables|Default|GetDistanceAlongSpline) SplineLength))))
    (:then_1
      (if (< (Variables|Default|GetDistanceAlongSpline) 0.0)
        (Variables|Default|SetDistanceAlongSpline (+ SplineLength (Variables|Default|GetDistanceAlongSpline)))))))

(fn UpdateDistanceAlongSpline
  (Variables|Default|SetDistanceAlongSpline (+ (* (Utilities|Time|GetWorldDeltaSeconds) (Variables|Default|GetTravelSpeed)) (Variables|Default|GetDistanceAlongSpline)))
  (CallFunction|ClampDistanceAlongSplne (Spline|GetSplineLength (Variables|/Game/BPs/BP_SplineActor.BP_SplineActor_C|GetSpline (Variables|Default|GetSplineActor)))))

(fn UpdateLocation
  (Transformation|SetActorLocation (Spline|GetLocationatDistanceAlongSpline (Variables|/Game/BPs/BP_SplineActor.BP_SplineActor_C|GetSpline (Variables|Default|GetSplineActor)) (Variables|Default|GetDistanceAlongSpline) "World") false false))

(fn UpdateRotation
  (Transformation|SetActorRotation (Spline|GetRotationatDistanceAlongSpline (Variables|/Game/BPs/BP_SplineActor.BP_SplineActor_C|GetSpline (Variables|Default|GetSplineActor)) (Variables|Default|GetDistanceAlongSpline) "World")))