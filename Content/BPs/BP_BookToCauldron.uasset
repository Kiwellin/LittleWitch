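; BP_BookToCauldron is an interactable book that, on its first interaction, travels along an assigned spline actor, presumably to a cauldron.
; A speed-scaled timeline drives position and rotation along the spline, then checks whether the book reached the end.
; If it has, the timeline reverses two seconds after the player character leaves the sphere.
; The construction script places the book at a spline offset and tints it through a dynamic material.
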(event OnComponentEndOverlap(Sphere)
  (params (OverlappedComponent :type Primitive%20Component%20Object%20Reference) (OtherActor :type Actor%20Object%20Reference) (OtherComp :type Primitive%20Component%20Object%20Reference) (OtherBodyIndex :type Integer))
  (Utilities|Casting|CastToBP_ThirdPersonCharacter OtherActor)
  (Utilities|FlowControl|Delay 2.0)
  (if (Variables|Default|GetHasreachedEndPoint)
    (bind _spline_ (Timeline|Timeline ReverseFromEnd)
      (:Update
        (Transformation|SetActorLocation (.Location (CallFunction|GetLocationandRotationfromSpline _spline_)) false false)
        (Transformation|SetActorRotation (.Rotation (CallFunction|GetLocationandRotationfromSpline _spline_))))
      (:Finished
        (CallFunction|CheckIFEnd)))))

(event Custom|MoveAlongSpline
  (Components|Timeline|SetPlayRate (Variables|Default|GetTimeline) (Variables|Default|GetSpeed))
  (bind _spline_ (Timeline|Timeline PlayFromStart)
    (:Update
      (Transformation|SetActorLocation (.Location (CallFunction|GetLocationandRotationfromSpline _spline_)) false false)
      (Transformation|SetActorRotation (.Rotation (CallFunction|GetLocationandRotationfromSpline _spline_))))
    (:Finished
      (CallFunction|CheckIFEnd))))

(event Custom|CheckIFEnd
  (if (Utilities|Operators|EqualEqual (Transformation|GetActorLocation) (.Location (CallFunction|GetLocationandRotationfromSpline 1.0)) 0.01)
    (Variables|Default|SetHasreachedEndPoint true)
    (else
      (Variables|Default|SetHasreachedEndPoint false))))

(event EventBeginPlay
  (Utilities|IsValid (Variables|Default|GetSplineActor)
    (:Is%20Valid
      (CallFunction|ApplyStartoffset))
    (:Is%20Not%20Valid
      (Development|PrintString "Spline not assigned"))))

(event Collision|EventActorBeginOverlap
  (params (OtherActor :type Actor%20Object%20Reference)))

(event EventTick
  (params (DeltaSeconds :type Float%20%28single-precision%29)))

(event EventInteract
  (if (not (Variables|Default|GetHasreachedEndPoint))
    (Utilities|FlowControl|DoOnce false
      (:Completed
        (CallFunction|MoveAlongSpline)
        (CallFunction|UpdateLocation)))))

(fn ConstructionScript
  (Utilities|IsValid (Variables|Default|GetMID)
    (:Is%20Valid
      _)
    (:Is%20Not%20Valid
      (bind _returnvalue (Rendering|Material|CreateDynamicMaterialInstance (Variables|Default|GetBook) 0 0 "None" :!class /Script/Engine.PrimitiveComponent))
      (Variables|Default|SetMID _returnvalue)))
  (Rendering|Material|SetScalarParameterValue (Variables|Default|GetMID) "HasColor" (CallFunction|Scalarvalueset (Variables|Default|GethasColor)) :!class /Script/Engine.MaterialInstanceDynamic)
  (Rendering|Material|SetVectorParameterValue (Variables|Default|GetMID) "Color" (Variables|Default|GetColor) :!class /Script/Engine.MaterialInstanceDynamic)
  (CallFunction|ApplyStartoffset)
  (CallFunction|UpdateRotation)
  (CallFunction|UpdateLocation))

(fn GetLocationandRotationfromSpline
  (params (A :type Float%20%28double-precision%29))
  (bind _splineactor (Variables|Default|GetSplineActor))
  (bind _spline (Variables|/Game/BPs/BP_SplineActor.BP_SplineActor_C|GetSpline _splineactor))
  (bind _returnvalue (Spline|GetSplineLength _spline))
  (bind _returnvalue_2 (* A _returnvalue))
  (return (Spline|GetLocationatDistanceAlongSpline _spline _returnvalue_2 "World") (Spline|GetRotationatDistanceAlongSpline _spline _returnvalue_2 "World")))

(fn ApplyStartoffset
  (Variables|Default|SetDistanceAlongSpline (* (Variables|Default|GetSplineOffset) (Spline|GetSplineLength (Variables|/Game/BPs/BP_SplineActor.BP_SplineActor_C|GetSpline (Variables|Default|GetSplineActor))))))

(fn Scalarvalueset
  (params (Condition :type Boolean))
  (if Condition
    (Variables|Default|SetScalarValue 1.0)
    (else
      (Variables|Default|SetScalarValue 0.0)))
  (return (Variables|Default|GetScalarValue)))

(fn UpdateLocation
  (Transformation|SetActorLocation (Spline|GetLocationatDistanceAlongSpline (Variables|/Game/BPs/BP_SplineActor.BP_SplineActor_C|GetSpline (Variables|Default|GetSplineActor)) (Variables|Default|GetDistanceAlongSpline) "World") false false))

(fn UpdateRotation
  (Transformation|SetActorRotation (Spline|GetRotationatDistanceAlongSpline (Variables|/Game/BPs/BP_SplineActor.BP_SplineActor_C|GetSpline (Variables|Default|GetSplineActor)) (Variables|Default|GetDistanceAlongSpline) "World")))