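; BP_SpellCard is a spell card actor whose paper glows when the player is nearby and looking at it.
; While active, Tick checks player distance and uses a dot product against the character's SpellCam forward vector to detect gaze.
; A timeline plays or reverses accordingly, driving EmissionStrength on the Paper's dynamic material during its play.
; InLOS and NotInLOS events also drive the timeline, while Interact is empty.
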(event Custom|InLOS
  (bind _newtrack_0 (Timeline|Timeline Play)
    (:Update
      (Rendering|Material|SetScalarParameterValue (Variables|Default|GetPaperMID) "EmissionStrength" _newtrack_0 :!class /Script/Engine.MaterialInstanceDynamic))))

(event Custom|NotInLOS
  (bind _newtrack_0 (Timeline|Timeline Reverse)
    (:Update
      (Rendering|Material|SetScalarParameterValue (Variables|Default|GetPaperMID) "EmissionStrength" _newtrack_0 :!class /Script/Engine.MaterialInstanceDynamic))))

(event EventBeginPlay
  (bind _asbp_third_person_character (Utilities|Casting|CastToBP_ThirdPersonCharacter (Game|GetPlayerCharacter 0)))
  (Variables|Default|SetAs%20BP%20Third%20Person%20Character _asbp_third_person_character)
  (bind _returnvalue (Rendering|Material|CreateDynamicMaterialInstance (Variables|Default|GetPaper) 0 0 "None" :!class /Script/Engine.PrimitiveComponent))
  (Variables|Default|SetPaperMID _returnvalue))

(event Collision|EventActorBeginOverlap
  (params (OtherActor :type Actor%20Object%20Reference)))

(event EventTick
  (params (DeltaSeconds :type Float%20%28single-precision%29))
  (if (Variables|Default|GetIsStillActive)
    (bind _returnvalue (CallFunction|DistancetoPlayer))
    (bind _is_true (CallFunction|DistanceLessThanXy _returnvalue))
    (if (and _is_true (CallFunction|IsPlayerLookingatObject))
      (bind _newtrack_0 (Timeline|Timeline Play)
        (:Update
          (Rendering|Material|SetScalarParameterValue (Variables|Default|GetPaperMID) "EmissionStrength" _newtrack_0 :!class /Script/Engine.MaterialInstanceDynamic)))
      (else
        (Timeline|Timeline Reverse)))))

(event EventInteract)

(fn ConstructionScript
  (|CallParentFunction))

(fn DistancetoPlayer
  (return (Math|Vector|VectorLength (- (Transformation|GetActorLocation) (Transformation|GetActorLocation (Game|Player|GetPlayerPawn 0))))))

(fn DistanceLessThanXy
  (params (value :type Float%20%28double-precision%29))
  (return (<= value (Variables|Default|GetMin%20Distance%20to%20Player))))

(fn IsPlayerLookingatObject
  (bind _as_bp_third_person_character (Variables|Default|GetAs%20BP%20Third%20Person%20Character))
  (bind _spellcam (Variables|/Game/BPs/BP_ThirdPersonCharacter.BP_ThirdPersonCharacter_C|GetSpellCam _as_bp_third_person_character))
  (return (>= (* (Math|Vector|DotProduct (Math|Vector|GetForwardVector (Math|Rotator|FindLookatRotation (Transformation|GetActorLocation self) (Transformation|GetWorldLocation _spellcam))) (Math|Vector|GetForwardVector _spellcam)) -1.0) 0.8)))