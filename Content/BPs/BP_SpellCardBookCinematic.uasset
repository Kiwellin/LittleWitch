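; Interactable spell card book that plays a one-shot Level Sequence cinematic.
; On Interact it disables player input, destroys its Sphere component, clears IsStillActive and zeroes the paper material's emission.
; It then plays the assigned sequence and re-enables input after a Delay matching the sequence's playback end time, rather than binding to a finished event.
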(event EventBeginPlay
  (|CallParentFunction) ; This node is disabled and will not be called.\nDrag off pins to build functionality.
)

(event Collision|EventActorBeginOverlap
  (params (OtherActor :type Actor%20Object%20Reference))
  (|CallParentFunction OtherActor) ; This node is disabled and will not be called.\nDrag off pins to build functionality.
)

(event EventTick
  (params (DeltaSeconds :type Float%20%28single-precision%29))
  (|CallParentFunction DeltaSeconds) ; This node is disabled and will not be called.\nDrag off pins to build functionality.
)

(event EventInteract
  (bind _returnvalue (Game|GetPlayerController 0))
  (bind _returnvalue_2 (Game|GetPlayerController 0))
  (bind _levelsequence (Variables|Default|GetLevelSequence))
  (bind _sequenceplayer (Variables|/Script/LevelSequence.LevelSequenceActor|GetSequencePlayer _levelsequence))
  (Input|DisableInput _returnvalue_2 _returnvalue_2)
  (Components|DestroyComponent (Variables|Default|GetSphere))
  (Variables|Default|SetIsStillActive false)
  (Rendering|Material|SetScalarParameterValue (Variables|Default|GetPaperMID) "EmissionStrength" 0.0 :!class /Script/Engine.MaterialInstanceDynamic)
  (Sequencer|Player|Play _sequenceplayer :!class /Script/MovieScene.MovieSceneSequencePlayer)
  (bind _returnvalue_3 (Class|MovieSceneSequenceExtensions|GetPlaybackEndSeconds (Class|MovieSceneSequencePlayer|GetSequence _sequenceplayer)))
  (Utilities|FlowControl|Delay _returnvalue_3)
  (Input|EnableInput _returnvalue _returnvalue))

(fn ConstructionScript
  (|CallParentFunction))