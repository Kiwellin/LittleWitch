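; BP_IngredientRoots is the roots ingredient, a collectible that is picked up and later delivered to a cauldron.
; Collected runs the parent logic, and both it and Delivered notify the character's CollectibleWidget through roots-specific calls.
; SequenceOnceDelivered passes its PlaySequence to the cauldron and activates it.
; EndScreen prints a debug "Hello" and opens the end screen level.
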(event Custom|EndScreen
  (Development|PrintString "Hello")
  (Game|OpenLevel(byObjectReference) "/Game/Maps/EndScreen.EndScreen"))

(event EventBeginPlay
  (|CallParentFunction) ; This node is disabled and will not be called.\nDrag off pins to build functionality.
)

(event Collision|EventActorBeginOverlap
  (params (OtherActor :type Actor%20Object%20Reference))
  (|CallParentFunction OtherActor) ; This node is disabled and will not be called.\nDrag off pins to build functionality.
)

(event EventTick
  (params (DeltaSeconds :type Float%20%28single-precision%29))
  (|CallParentFunction DeltaSeconds) ; This node is disabled and will not be called.\nDrag off pins to build functionality.
)

(event EventSequenceOnceDelivered
  (params (Cauldron :type BP%20Cauldron%20Object%20Reference))
  (Variables|/Game/BPs/BP_Cauldron.BP_Cauldron_C|SetCurrentSequence Cauldron (Variables|Default|GetPlaySequence))
  (Default|ActivateSequence Cauldron))

(event EventCollected
  (params (ThirdPersonCharacter :type BP%20Third%20Person%20Character%20Object%20Reference))
  (|CallParentFunction 0)
  (Default|OnCollectedRoots (Variables|/Game/BPs/BP_ThirdPersonCharacter.BP_ThirdPersonCharacter_C|GetCollectibleWidget ThirdPersonCharacter)))

(event EventDelivered
  (params (chara :type BP%20Third%20Person%20Character%20Object%20Reference))
  (Default|RootsDelivered (Variables|/Game/BPs/BP_ThirdPersonCharacter.BP_ThirdPersonCharacter_C|GetCollectibleWidget chara)))

(fn ConstructionScript
  (|CallParentFunction))