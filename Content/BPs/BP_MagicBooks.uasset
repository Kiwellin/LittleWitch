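; BP_MagicBooks is a magic book that, on Activate, moves between two points and changes the jump power of a player on it.
; A speed-scaled timeline lerps the Pivot from Start to End and the character's JumpZVelocity from default toward JumpVelocity.
; Box overlaps track the third-person character and restore default jump velocity on exit.
; The construction script applies optional color through a dynamic material instance.
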(event OnComponentBeginOverlap(Box)
  (params (OverlappedComponent :type Primitive%20Component%20Object%20Reference) (OtherActor :type Actor%20Object%20Reference) (OtherComp :type Primitive%20Component%20Object%20Reference) (OtherBodyIndex :type Integer) (bFromSweep :type Boolean) (SweepResult :type Hit%20Result%20Structure%20%28by%20ref%29))
  (bind _asbp_third_person_character (Utilities|Casting|CastToBP_ThirdPersonCharacter OtherActor))
  (Variables|Default|SetAs%20BP%20Third%20Person%20Character _asbp_third_person_character)
  (Variables|Default|SetIsPlayerOn true))

(event OnComponentEndOverlap(Box)
  (params (OverlappedComponent :type Primitive%20Component%20Object%20Reference) (OtherActor :type Actor%20Object%20Reference) (OtherComp :type Primitive%20Component%20Object%20Reference) (OtherBodyIndex :type Integer))
  (bind _asbp_third_person_character (Utilities|Casting|CastToBP_ThirdPersonCharacter OtherActor))
  (Variables|/Script/Engine.CharacterMovementComponent|SetJumpZVelocity (Variables|/Script/Engine.Character|GetCharacterMovement _asbp_third_person_character) (Variables|/Game/BPs/BP_ThirdPersonCharacter.BP_ThirdPersonCharacter_C|GetDefaultJumpVelocity _asbp_third_person_character))
  (Variables|Default|SetIsPlayerOn false))

(event Custom|Activate
  (bind _as_bp_third_person_character (Variables|Default|GetAs%20BP%20Third%20Person%20Character))
  (Components|Timeline|SetPlayRate (Variables|Default|GetTimeline) (Variables|Default|GetSpeed))
  (bind _newtrack_1 (Timeline|Timeline PlayFromStart)
    (:Update
      (Transformation|SetRelativeTransform (Variables|Default|GetPivot) (Math|Transform|MakeTransform (Math|Vector|Lerp(Vector) (Variables|/Script/Engine.SceneComponent|GetRelativeLocation (Variables|Default|Getstart)) (Variables|/Script/Engine.SceneComponent|GetRelativeLocation (Variables|Default|Getend)) _newtrack_1) "0, 0, 0" "1.000000,1.000000,1.000000") false false)
      (Utilities|IsValid _as_bp_third_person_character
        (:Is%20Valid
          (if (Variables|Default|GetIsPlayerOn)
            (Variables|/Script/Engine.CharacterMovementComponent|SetJumpZVelocity (Variables|/Script/Engine.Character|GetCharacterMovement _as_bp_third_person_character) (Math|Float|Lerp (* (Variables|/Game/BPs/BP_ThirdPersonCharacter.BP_ThirdPersonCharacter_C|GetDefaultJumpVelocity _as_bp_third_person_character) 1.0) (Variables|Default|GetJumpVelocity) _newtrack_1))))))))

(event EventBeginPlay)

(event Collision|EventActorBeginOverlap
  (params (OtherActor :type Actor%20Object%20Reference)))

(event EventTick
  (params (DeltaSeconds :type Float%20%28single-precision%29)))

(fn ConstructionScript
  (Utilities|IsValid (Variables|Default|GetMID)
    (:Is%20Valid
      _)
    (:Is%20Not%20Valid
      (bind _returnvalue (Rendering|Material|CreateDynamicMaterialInstance (Variables|Default|GetBook_ClosedMagic) 0 0 "None" :!class /Script/Engine.PrimitiveComponent))
      (Variables|Default|SetMID _returnvalue)))
  (Rendering|Material|SetScalarParameterValue (Variables|Default|GetMID) "HasColor" (CallFunction|Scalarvalueset (Variables|Default|GethasColor)) :!class /Script/Engine.MaterialInstanceDynamic)
  (Rendering|Material|SetVectorParameterValue (Variables|Default|GetMID) "Color" (Variables|Default|GetColor) :!class /Script/Engine.MaterialInstanceDynamic))

(fn Scalarvalueset
  (params (Condition :type Boolean))
  (if Condition
    (Variables|Default|SetScalarValue 1.0)
    (else
      (Variables|Default|SetScalarValue 0.0)))
  (return (Variables|Default|GetScalarValue)))