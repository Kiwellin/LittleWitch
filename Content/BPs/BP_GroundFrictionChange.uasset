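; BP_GroundFrictionChange is a zone actor that changes the ground handling of BP_ThirdPersonCharacter while it overlaps, such as for slippery or sticky surfaces.
; On begin overlap it caches the character's braking friction, braking deceleration and ground friction, then applies its own values to CharacterMovement.
; On end overlap it restores the cached values, which live in a single set of variables on the actor rather than per character.
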(event EventBeginPlay)

(event Collision|EventActorBeginOverlap
  (params (OtherActor :type Actor%20Object%20Reference))
  (bind _asbp_third_person_character (Utilities|Casting|CastToBP_ThirdPersonCharacter OtherActor))
  (Variables|Default|SetDefaultBraking%20Friction (Variables|/Script/Engine.CharacterMovementComponent|GetBrakingFriction (Variables|/Script/Engine.Character|GetCharacterMovement _asbp_third_person_character)))
  (Variables|Default|SetDefaultBraking%20Deceleration%20Walking (Variables|/Script/Engine.CharacterMovementComponent|GetBrakingDecelerationWalking (Variables|/Script/Engine.Character|GetCharacterMovement _asbp_third_person_character)))
  (Variables|Default|SetCharacterDefaultFriction (Variables|/Script/Engine.CharacterMovementComponent|GetGroundFriction (Variables|/Script/Engine.Character|GetCharacterMovement _asbp_third_person_character)))
  (Variables|/Script/Engine.CharacterMovementComponent|SetBrakingFriction (Variables|/Script/Engine.Character|GetCharacterMovement _asbp_third_person_character) (Variables|Default|GetBraking%20Friction))
  (Variables|/Script/Engine.CharacterMovementComponent|SetBrakingDecelerationWalking (Variables|/Script/Engine.Character|GetCharacterMovement _asbp_third_person_character) (Variables|Default|GetBraking%20Deceleration%20Walking))
  (Variables|/Script/Engine.CharacterMovementComponent|SetGroundFriction (Variables|/Script/Engine.Character|GetCharacterMovement _asbp_third_person_character) (Variables|Default|GetGroundFriction)))

(event EventTick
  (params (DeltaSeconds :type Float%20%28single-precision%29)))

(event Collision|EventActorEndOverlap
  (params (OtherActor :type Actor%20Object%20Reference))
  (bind _asbp_third_person_character (Utilities|Casting|CastToBP_ThirdPersonCharacter OtherActor))
  (Variables|/Script/Engine.CharacterMovementComponent|SetBrakingFriction (Variables|/Script/Engine.Character|GetCharacterMovement _asbp_third_person_character) (Variables|Default|GetDefaultBraking%20Friction))
  (Variables|/Script/Engine.CharacterMovementComponent|SetBrakingDecelerationWalking (Variables|/Script/Engine.Character|GetCharacterMovement _asbp_third_person_character) (Variables|Default|GetDefaultBraking%20Deceleration%20Walking))
  (Variables|/Script/Engine.CharacterMovementComponent|SetGroundFriction (Variables|/Script/Engine.Character|GetCharacterMovement _asbp_third_person_character) (Variables|Default|GetCharacterDefaultFriction)))

(fn ConstructionScript)