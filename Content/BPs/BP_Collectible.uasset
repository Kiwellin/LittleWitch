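; BP_Collectible is a spinning crystal pickup that BP_ThirdPersonCharacter collects once by overlapping it.
; Tick idly rotates the Pivot; on overlap, a Timeline lifts, spins and scales it while driving the crystal's emissive through a dynamic material instance, then destroys the actor.
; OnCollected receives the collecting character but only prints a debug string, apparently a hook for child collectibles.
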(event Custom|PlayCollectAnimation
  (bind _pivot (Variables|Default|GetPivot))
  (bind (_direction _zmovement _rotationspeed _size _light) (Timeline|Timeline Play)
    (:Update
      (Transformation|SetRelativeLocation (Variables|Default|GetPivot) (Math|Vector|MakeVector 0.0 0.0 (* _zmovement (Variables|Default|GetAnimZDist))) false false)
      (Transformation|AddRelativeRotation _pivot (Math|Rotator|MakeRotator 0.0 0.0 (* _rotationspeed (Variables|Default|GetAnim%20Rot%20Speed) (Utilities|Time|GetWorldDeltaSeconds))) false false)
      (Transformation|SetRelativeScale3D _pivot (* _size "1.000000,1.000000,1.000000"))
      (Rendering|Material|SetScalarParameterValue (Variables|Default|GetMIDCrystal) "EmissMulti" (* _light (Variables|Default|GetMIDEmis)) :!class /Script/Engine.MaterialInstanceDynamic))
    (:Finished
      (Actor|DestroyActor))))

(event Custom|OnCollected
  (params (ThirdPersonCharacter :type BP%20Third%20Person%20Character%20Object%20Reference))
  (Development|PrintString "CollecteCollecetible"))

(event EventTick
  (params (DeltaSeconds :type Float%20%28single-precision%29))
  (Transformation|AddRelativeRotation (Variables|Default|GetPivot) (Math|Rotator|MakeRotator 0.0 0.0 (* (Variables|Default|GetIdle%20Rot%20Speed) (Utilities|Time|GetWorldDeltaSeconds))) false false))

(event Collision|EventActorBeginOverlap
  (params (OtherActor :type Actor%20Object%20Reference))
  (bind _asbp_third_person_character (Utilities|Casting|CastToBP_ThirdPersonCharacter OtherActor))
  (Utilities|FlowControl|DoOnce false
    (:Completed
      (CallFunction|PlayCollectAnimation)
      (CallFunction|OnCollected _asbp_third_person_character))))

(event EventBeginPlay
  (bind _returnvalue (Rendering|Material|CreateDynamicMaterialInstance (Variables|Default|GetCrystalShards) 0 0 "None" :!class /Script/Engine.PrimitiveComponent))
  (bind _output_get (Variables|Default|SetMIDCrystal _returnvalue))
  (bind _returnvalue_2 (Rendering|Material|GetScalarParameterValue _output_get "EmissMulti" :!class /Script/Engine.MaterialInstanceDynamic))
  (Variables|Default|SetMIDEmis _returnvalue_2))

(fn ConstructionScript)