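; BP_IngredientHerbs is the herbs ingredient, a collectible that the player picks up and delivers to a cauldron.
; Its collect and deliver events notify the character's CollectibleWidget through herb-specific calls.
; A post-delivery event assigns its PlaySequence to the cauldron's current sequence and activates it.
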(event EventBeginPlay
  (|CallParentFunction) ; This node is disabled and will not be called.\nDrag off pins to build functionality.
)

(event Collision|EventActorBeginOverlap
  (params (OtherActor :type Actor%20Object%20Reference))
  (|CallParentFunction OtherActor) ; This node is disabled and will not be called.\nDrag off pins to build functionality.
)

(event EventTick
  (params (DeltaSeconds :type Float%20%28single-precision%29))
  (|CallParentFunction DeltaSeconds) ; This node is disabled and will not be called.\nDrag off pins to build functionality.
)

(event EventSequenceOnceDelivered
  (params (Cauldron :type BP%20Cauldron%20Object%20Reference))
  (Variables|/Game/BPs/BP_Cauldron.BP_Cauldron_C|SetCurrentSequence Cauldron (Variables|Default|GetPlaySequence))
  (Default|ActivateSequence Cauldron))

(event EventDelivered
  (params (chara :type BP%20Third%20Person%20Character%20Object%20Reference))
  (Default|HerbsDelivered (Variables|/Game/BPs/BP_ThirdPersonCharacter.BP_ThirdPersonCharacter_C|GetCollectibleWidget chara)))

(event EventCollected
  (params (ThirdPersonCharacter :type BP%20Third%20Person%20Character%20Object%20Reference))
  (Default|OnCollectedHerbs (Variables|/Game/BPs/BP_ThirdPersonCharacter.BP_ThirdPersonCharacter_C|GetCollectibleWidget ThirdPersonCharacter)))

(fn ConstructionScript
  (|CallParentFunction))