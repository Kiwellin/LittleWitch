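; BP_InteractablePlatform is an interactable platform that moves once along a configured direction when interacted with.
; On the first Interact, a timeline drives the Pivot component's relative location from its track value times the normalized Direction and Distance.
; A DoOnce gate with no reset keeps it from triggering again, and the construction script only calls its parent.
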(event EventInteract
  (Utilities|FlowControl|DoOnce false
    (:Completed
      (bind _newtrack_1 (Timeline|Timeline Play)
        (:Update
          (Transformation|SetRelativeTransform (Variables|Default|Getpivot) (Math|Transform|MakeTransform (* (* _newtrack_1 (Math|Vector|Normalize (Variables|Default|GetDirection))) (Variables|Default|GetDistance)) "0, 0, 0" "1.000000,1.000000,1.000000") false false))))))

(fn ConstructionScript
  (|CallParentFunction))