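; Platform actor that moves along the spline of an assigned SplineActor, starting on BeginPlay.
; A Timeline with play rate set by Speed drives a fraction of spline length, setting the Pivot component's world location and rotation each update without sweep.
; An on-screen error prints if no spline actor is assigned.
; Tick, UpdateDistanceAlongSpline and the TravelSpeed-based distance logic are unused leftovers.
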(event Custom|MoveAlongSpline
  (bind _splineactor (Variables|Default|GetSplineActor))
  (bind _spline (Variables|/Game/BPs/BP_SplineActor.BP_SplineActor_C|GetSpline _splineactor))
  (Components|Timeline|SetPlayRate (Variables|Default|GetTimeline) (Variables|Default|GetSpeed))
  (bind _newtrack_1 (Timeline|Timeline Play)
    (:Update
      (Transformation|SetWorldLocation (Variables|Default|Getpivot) (Spline|GetLocationatDistanceAlongSpline _spline (* _newtrack_1 (Spline|GetSplineLength _spline)) "World") false false)
      (Transformation|SetWorldRotation (Variables|Default|Getpivot) (Spline|GetRotationatDistanceAlongSpline _spline (* _newtrack_1 (Spline|GetSplineLength _spline)) "World") false false))))

(event EventBeginPlay
  (Utilities|IsValid (Variables|Default|GetSplineActor)
    (:Is%20Valid
      (CallFunction|MoveAlongSpline))
    (:Is%20Not%20Valid
      (Development|PrintString "SplineActorIsNotAssigned" true true "(R=1.000000,G=0.080729,B=0.222796,A=1.000000)" 12.0))))

(event EventTick
  (params (DeltaSeconds :type Float%20%28single-precision%29)))

(fn ConstructionScript)

(fn UpdateDistanceAlongSpline)