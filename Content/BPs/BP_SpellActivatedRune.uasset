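; BP_SpellActivatedRune is a rune actor that lights up and becomes visible when the player is near and looking at it.
; Each tick it checks the distance to the player and a dot product between the SpellCam's forward vector and its direction to the rune.
; The Emission timeline plays or reverses accordingly, driving emission and opacity on a dynamic material.
; InLOS and NotInLOS events drive the same timeline; spell-projectile handling is unconnected.
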(event Custom|InLOS
  (bind _newtrack_0 (Timeline|emission Play)
    (:Update
      (Rendering|Material|SetScalarParameterValue (Variables|Default|GetRuneMID) "EmissionStrength" _newtrack_0 :!class /Script/Engine.MaterialInstanceDynamic)
      (Rendering|Material|SetScalarParameterValue (Variables|Default|GetRuneMID) "Opacity" _newtrack_0 :!class /Script/Engine.MaterialInstanceDynamic))))

(event Custom|NotInLOS
  (bind _newtrack_0 (Timeline|emission Reverse)
    (:Update
      (Rendering|Material|SetScalarParameterValue (Variables|Default|GetRuneMID) "EmissionStrength" _newtrack_0 :!class /Script/Engine.MaterialInstanceDynamic)
      (Rendering|Material|SetScalarParameterValue (Variables|Default|GetRuneMID) "Opacity" _newtrack_0 :!class /Script/Engine.MaterialInstanceDynamic))))

(event EventTick
  (params (DeltaSeconds :type Float%20%28single-precision%29))
  (bind _returnvalue (CallFunction|GetDistancetoPlayer))
  (bind _returnvalue1 (CallFunction|DistanceLessThanXY _returnvalue))
  (if (and _returnvalue1 (CallFunction|IsPlayerLookingatObject))
    (bind _newtrack_0 (Timeline|emission Play)
      (:Update
        (Rendering|Material|SetScalarParameterValue (Variables|Default|GetRuneMID) "EmissionStrength" _newtrack_0 :!class /Script/Engine.MaterialInstanceDynamic)
        (Rendering|Material|SetScalarParameterValue (Variables|Default|GetRuneMID) "Opacity" _newtrack_0 :!class /Script/Engine.MaterialInstanceDynamic)))
    (else
      (Timeline|emission Reverse))))

(event EventBeginPlay
  (bind _returnvalue (Rendering|Material|CreateDynamicMaterialInstance (Variables|Default|GetRune) 0 0 "None" :!class /Script/Engine.PrimitiveComponent))
  (Variables|Default|SetRuneMID _returnvalue)
  (bind _asbp_third_person_character (Utilities|Casting|CastToBP_ThirdPersonCharacter (Game|Player|GetPlayerPawn 0)))
  (Variables|Default|SetAs%20BP%20Third%20Person%20Character _asbp_third_person_character))

(fn ConstructionScript)

(fn GetDistancetoPlayer
  (return (Math|Vector|VectorLength (- (Transformation|GetActorLocation) (Transformation|GetActorLocation (Game|Player|GetPlayerPawn 0))))))

(fn DistanceLessThanXY
  (params (NewParam :type Float%20%28double-precision%29))
  (return (<= NewParam (Variables|Default|GetMin%20DistanceToPlayer))))

(fn IsPlayerLookingatObject
  (bind _as_bp_third_person_character (Variables|Default|GetAs%20BP%20Third%20Person%20Character))
  (bind _spellcam (Variables|/Game/BPs/BP_ThirdPersonCharacter.BP_ThirdPersonCharacter_C|GetSpellCam _as_bp_third_person_character))
  (return (>= (* (Math|Vector|DotProduct (Math|Vector|GetForwardVector (Math|Rotator|FindLookatRotation (Transformation|GetActorLocation self) (Transformation|GetWorldLocation _spellcam))) (Math|Vector|GetForwardVector _spellcam)) -1.0) 0.8)))