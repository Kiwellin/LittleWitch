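; BP_StoneInteractable is an interactable stone whose emissive glow toggles on and off.
; BeginPlay creates a dynamic material instance on the first material slot of the stone mesh.
; Interact flips EmissionStrength by subtracting it from MaxEmission, then writes the result to the material's scalar parameter.
; IsOn reports the state by testing whether EmissionStrength equals MaxEmission.
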(event EventBeginPlay
  (bind _returnvalue (Rendering|Material|CreateDynamicMaterialInstance (Variables|Default|GetStones_SM_Stone_003) 0 0 "None" :!class /Script/Engine.PrimitiveComponent))
  (Variables|Default|SetMID_0 _returnvalue))

(event Collision|EventActorBeginOverlap
  (params (OtherActor :type Actor%20Object%20Reference)))

(event EventTick
  (params (DeltaSeconds :type Float%20%28single-precision%29)))

(event EventInteract
  (bind _output_get (Variables|Default|SetEmissionStrength (- (Variables|Default|GetMaxEmission) (Variables|Default|GetEmissionStrength))))
  (Rendering|Material|SetScalarParameterValue (Variables|Default|GetMID_0) "EmissionStrength" _output_get :!class /Script/Engine.MaterialInstanceDynamic))

(fn ConstructionScript
  (|CallParentFunction))

(fn Ison
  (return (== (Variables|Default|GetEmissionStrength) (Variables|Default|GetMaxEmission))))