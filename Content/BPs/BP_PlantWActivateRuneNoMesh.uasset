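; Rune-activated plant whose Target component, when hit by a fire arrow, opens the attached leaf actors and is then destroyed.
; On BeginPlay it gathers directly attached actors and passes its LaunchVelocity to each BP_Leafs among them.
; Activation sets the open flags on each leaf and its anim instance.
; Both passes use a local delayed ForEach macro to stagger the leaves over time.
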(event OnComponentHit(Target)
  (params (HitComponent :type Primitive%20Component%20Object%20Reference) (OtherActor :type Actor%20Object%20Reference) (OtherComp :type Primitive%20Component%20Object%20Reference) (NormalImpulse :type Vector :default "0, 0, 0") (Hit :type Hit%20Result%20Structure%20%28by%20ref%29))
  (Utilities|Casting|CastToBP_ProjectileFireArrow OtherActor)
  (CallFunction|Active)
  (Components|DestroyComponent (Variables|Default|GetTarget)))

(event Custom|Active
  (bind _arrayelement (Utilities|ForEachLoopWDelay (Variables|Default|GetOut%20Actors) 0.5)
    (:LoopBody
      (bind _asbp_leafs (Utilities|Casting|CastToBP_Leafs _arrayelement))
      (bind _asabp_test_leaf (Utilities|Casting|CastToABP_TestLeaf (Components|SkeletalMesh|GetAnimInstance (Variables|/Game/BPs/BP_Leafs.BP_Leafs_C|GetTestLeaf _asbp_leafs))))
      (Variables|/Game/Assets/AnimatedLeafs/ABP_TestLeaf.ABP_TestLeaf_C|SetLeafOpen _asabp_test_leaf true)
      (Variables|/Game/BPs/BP_Leafs.BP_Leafs_C|SetLeafsOpen _asbp_leafs true))))

(event EventBeginPlay
  (bind _output_get (Variables|Default|SetOut%20Actors (Actor|GetAttachedActors true false)))
  (bind _arrayelement (Utilities|ForEachLoopWDelay _output_get 0.2)
    (:LoopBody
      (bind _asbp_leafs (Utilities|Casting|CastToBP_Leafs _arrayelement))
      (Variables|/Game/BPs/BP_Leafs.BP_Leafs_C|SetLaunch%20Velocity _asbp_leafs (Variables|Default|GetLaunch%20Velocity)))))

(event Collision|EventActorBeginOverlap
  (params (OtherActor :type Actor%20Object%20Reference)))

(event EventTick
  (params (DeltaSeconds :type Float%20%28single-precision%29)))

(fn ConstructionScript)