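; BP_Respawnpoint is a checkpoint actor that registers itself as the player character's respawn point when an overlap begins.
; The overlap handler casts player pawn 0 without checking the overlapping actor, then after a short delay activates FXSpawn and plays a timeline driving emission strength.
; The construction script creates the Cube's dynamic material instance for that glow.
; GetRespawnLocation returns the RespawnPivot's world location and rotation.
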(event Collision|EventActorBeginOverlap
  (params (OtherActor :type Actor%20Object%20Reference))
  (bind _asbp_third_person_character (Utilities|Casting|CastToBP_ThirdPersonCharacter (Game|Player|GetPlayerPawn 0)))
  (Variables|/Game/BPs/BP_ThirdPersonCharacter.BP_ThirdPersonCharacter_C|SetMyRespawnPoint _asbp_third_person_character self)
  (Utilities|FlowControl|Delay 0.2)
  (Components|Activation|Activate (Variables|Default|GetFX_Spawn) true)
  (bind _emiss (Timeline|SpawnEmiss PlayFromStart)
    (:Update
      (Rendering|Material|SetScalarParameterValue (Variables|Default|GetMIDSpawn) "EmissionStrength" _emiss :!class /Script/Engine.MaterialInstanceDynamic))))

(fn ConstructionScript
  (Utilities|IsValid (Variables|Default|GetMIDSpawn)
    (:Is%20Not%20Valid
      (bind _returnvalue (Rendering|Material|CreateDynamicMaterialInstance (Variables|Default|GetCube) 0 0 "None" :!class /Script/Engine.PrimitiveComponent))
      (Variables|Default|SetMIDSpawn _returnvalue))))

(fn GetRespawnLocation
  (bind _respawnpivot (Variables|Default|GetRespawnPivot))
  (return (Transformation|GetWorldLocation _respawnpivot) (Transformation|GetWorldRotation _respawnpivot)))